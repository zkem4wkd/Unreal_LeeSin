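; Enemy character Blueprint that reacts to R and Q effects, mainly chaining airborne hits between enemies.
; While IsRAirborne is set, overlapping another Char_Enemy damages it, zeroes its velocity, launches it upward with a hit emitter, then zeroes velocity again after a delay.
; ActiveParticle shows the Q부착후보 particle until a timer deactivates it.
; BeginPlay, Tick and SetMoveSpeed are empty; the walk-speed logic is disconnected.
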(event `self.ReceiveBeginPlay`)

(event `SetMoveSpeed`)

(event `self.ReceiveTick`
  (params (DeltaSeconds :type "Float (single-precision)")))

(event `self.ReceiveActorBeginOverlap`
  (params (OtherActor :type "Actor Object Reference"))
  (if (`self.is_R_Airborne`)
    (bind _aschar_enemy (cast `/Game/BluePrint/Enemy/Char_Enemy` OtherActor))
    (`GameplayStatics.ApplyDamage` _aschar_enemy 10.0)
    (bind _capsulecomponent (`Character.CapsuleComponent` _aschar_enemy))
    (`PrimitiveComponent.SetPhysicsLinearVelocity` _capsulecomponent (0.0 0.0 0.0) false "None")
    (`self.LaunchCharacter` _aschar_enemy (0.0 0.0 700.0) false false)
    (`GameplayStatics.SpawnEmitterAttached` "/Game/FXVarietyPack/Particles/P_ky_hit2.P_ky_hit2" _capsulecomponent)
    (`KismetSystemLibrary.Delay` 1.0)
    (`PrimitiveComponent.SetPhysicsLinearVelocity` _capsulecomponent (0.0 0.0 0.0) false "None")))

(event `ActiveParticle`
  (`ActorComponent.SetActive` (`self.q부착후보`) true false)
  (`KismetSystemLibrary.K2_SetTimer` null "DeactivateParticle" 2.5))

(event `DeactivateParticle`
  (`ActorComponent.Deactivate` (`self.q부착후보`)))

(event `OnTakeAnyDamage_이벤트` :!signature `self.OnTakeAnyDamage`
  (params (DamagedActor :type "Actor Object Reference") (Damage :type "Float (single-precision)") (DamageType :type "DamageType Object Reference") (InstigatedBy :type "Controller Object Reference") (DamageCauser :type "Actor Object Reference"))
  (add `self.OnTakeAnyDamage` (delegate `OnTakeAnyDamage_이벤트`)))

(fn `UserConstructionScript`)