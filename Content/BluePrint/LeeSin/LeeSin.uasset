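; Player Lee Sin character Blueprint handling cursor-targeted basic attacks and the champion's Q/W/E/R skills.
; Q spawns a LeeSin_Q projectile, then dashes on a hit; W dashes to allies or self-casts, recasting to change attack delay.
; E damages nearby enemies, recasting to slow; R knocks a target back, damaging enemies along a sphere-traced path.
; State flags gate recasts, timers reset cooldowns, and SkillUIWidget displays skill state.
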(event `Key|RightMouseButton`
  (params (Key :type "Key Structure"))
  (bind (_bblockinghit _binitialoverlap _time _distance _location _impactpoint _normal _impactnormal _physmat _hitactor) (`GameplayStatics.BreakHitResult` (`PlayerController.GetHitResultUnderCursorByChannel` (`GameplayStatics.GetPlayerController` 0) "TraceTypeQuery1" true)))
  ;[1 1 1] 기본공격
  (:`Pressed`
    (bind _aschar_enemy (cast `/Game/BluePrint/Enemy/Char_Enemy` _hitactor :!label _label))
    (if (== _hitactor _aschar_enemy)
      (bind _output_get (set `self.TargetEnemy` _aschar_enemy))
      (if (<= (`self.GetDistanceTo` _output_get) (`self.NormalAttackRange`))
        (bind (_returnvalue_roll _returnvalue_pitch _returnvalue_yaw) (`KismetMathLibrary.BreakRotator` (`KismetMathLibrary.FindLookAtRotation` (`self.K2_GetActorLocation`) (`self.K2_GetActorLocation` _output_get))))
        (`self.K2_SetActorRotation` (`KismetMathLibrary.MakeRotator` 0.0 0.0 _returnvalue_yaw))
        (if (`self.IsNormalAttackDelay`)
          (`self.PlayAnimMontage` "/Game/BluePrint/LeeSin/Animation/LeeSin_NormalAttack_AniMontage.LeeSin_NormalAttack_AniMontage")
          (`GameplayStatics.ApplyDamage` _output_get 3.0)
          (`|ExecutionSequence`
            (:`then_0`
              (set `self.IsNormalAttackMode` false)
              (set `self.IsNormalAttackDelay` false)
              (`KismetSystemLibrary.Delay` (`self.NormalAttackDelay`))
              (set `self.IsNormalAttackDelay` true))
            (:`then_1`
              (`KismetSystemLibrary.Delay` 0.3)
              (`GameplayStatics.SpawnEmitterAttached` "/Game/FXVarietyPack/Particles/P_ky_hit2.P_ky_hit2" (`Actor.RootComponent` _output_get) "None" (0.0 0.0 0.0) (struct) (0.5 0.5 0.5)))))
        (else
          (`AIBlueprintHelperLibrary.SimpleMoveToActor` (`self.GetController`) _output_get))))))

(event `Key|A`
  (params (Key :type "Key Structure"))
  ;[1 1 1] 기본공격
  (:`Pressed`
    (set `self.IsNormalAttackMode` true)))

(event `Key|LeftMouseButton`
  (params (Key :type "Key Structure"))
  ;[1 1 1] 기본공격
  (:`Pressed`
    (if (`self.IsNormalAttackMode`)
      (goto _label))))

(event `Key|Q`
  (params (Key :type "Key Structure"))
  (bind _returnvalue (`self.K2_GetActorLocation`))
  (bind _returnvalue_2 (`self.K2_GetActorLocation`))
  (bind _skilluireference (`self.SkillUIReference`))
  (bind _capsulecomponent (`self.CapsuleComponent`))
  (bind _returnvalue_3 (`self.K2_GetActorLocation` (`self.TargetActor`)))
  (bind (_bblockinghit _binitialoverlap _time _distance _location) (`GameplayStatics.BreakHitResult` (`PlayerController.GetHitResultUnderCursorByChannel` (`GameplayStatics.GetPlayerController` 0) "TraceTypeQuery1" true)))
  (bind (_returnvalue_roll _returnvalue_pitch _returnvalue_yaw) (`KismetMathLibrary.BreakRotator` (`KismetMathLibrary.FindLookAtRotation` _returnvalue _returnvalue_3)))
  (bind (_returnvalue_roll_2 _returnvalue_pitch_2 _returnvalue_yaw_2) (`KismetMathLibrary.BreakRotator` (`KismetMathLibrary.FindLookAtRotation` _returnvalue_2 _location)))
  (bind _returnvalue_4 (`KismetMathLibrary.MakeRotator` 0.0 0.0 _returnvalue_yaw))
  (bind _returnvalue_5 (* (`KismetMathLibrary.Vector_Distance` _returnvalue_3 _returnvalue) 0.001))
  ;[1 1 1] Q
  ;;[1 1 1] 스킬 쿨타임
  (:`Pressed`
    ;;;[1 1 1 1 14] Q를 이미 맞춘 상대인지 체크
    (if (`self.IsSonicWaveHit`)
      ;;[1 1 1] Q 맞춘 상태면 공명의 일격 날아가기
      (if (`self.IsValid`)
        (`|ExecutionSequence`
          (:`then_0`
            (`KismetSystemLibrary.MoveComponentTo` _capsulecomponent (- _returnvalue_3 (`KismetMathLibrary.Normal` (- _returnvalue_3 _returnvalue))) _returnvalue_4 false false _returnvalue_5)
            (set `self.IsSonicWaveHit` false)
            (`MovementComponent.StopMovementImmediately` (`self.CharacterMovement`))
            (`GameplayStatics.SpawnEmitterAttached` "/Game/FXVarietyPack/Particles/P_ky_hit2.P_ky_hit2" _capsulecomponent))
          (:`then_1`
            (`self.K2_SetActorRotation` _returnvalue_4)
            (`self.PlayAnimMontage` "/Game/BluePrint/LeeSin/Animation/LeeSin_QSkill2_Move_AniMontage1.LeeSin_QSkill2_Move_AniMontage1" (/ 0.25 _returnvalue_5))
            (`GameplayStatics.PlaySoundAtLocation` "/Game/BluePrint/LeeSin/Sound/q_날아감.q_날아감" _returnvalue (struct) 1.0 1.0 0.0 null null null null)
            (`Image.SetColorAndOpacity` (`/Game/BluePrint/UI/SkillUIWidget.Q_SkillImage_2` (`self.SkillUIReference`)) (make `LinearColor` 0.0 0.0 0.0)))))
      (elif (`self.CanUseSkill_Q`)
        (`|SpawnActorFromClass` "/Game/BluePrint/LeeSin/Skill/LeeSin_Q.LeeSin_Q_C" (`KismetMathLibrary.MakeTransform` (`self.K2_GetActorLocation`) (`KismetMathLibrary.MakeRotFromX` (`KismetMathLibrary.Normal` (- _location _returnvalue_2)))) "Undefined" "MultiplyWithRoot" null null)
        (`|ExecutionSequence`
          (:`then_0`
            (set `self.CanUseSkill_Q` false)
            (`KismetSystemLibrary.K2_SetTimer` null "ResetQSkillCoolTime" (`self.Skill_Q_CoolTime`)))
          (:`then_1`
            ;;[1 1 1] 스킬 사용할 때 캐릭터 방향 회전
            (`self.K2_SetActorRotation` (`KismetMathLibrary.MakeRotator` 0.0 0.0 _returnvalue_yaw_2))
            (`self.PlayAnimMontage` "/Game/BluePrint/LeeSin/Animation/LeeSin_QSkill_AniMontage.LeeSin_QSkill_AniMontage" 1.5))
          (:`then_2`
            (`/Game/BluePrint/UI/SkillUIWidget.StartQCoolDown` _skilluireference)
            (`/Game/BluePrint/UI/SkillUIWidget.UpdateCoolDown` _skilluireference)))
        (else
          (`KismetSystemLibrary.PrintText` "Q 스킬 쿨타임"))))))

(event `ResetQSkillCoolTime`
  ;[1 1 1] Q
  ;;[1 1 1] 스킬 쿨타임
  (set `self.CanUseSkill_Q` true))

(event `self.ReceiveBeginPlay`
  (bind _returnvalue (`|CreateWidget` "/Game/BluePrint/UI/SkillUIWidget.SkillUIWidget_C"))
  (bind _output_get (set `self.SkillUIReference` _returnvalue))
  (`UserWidget.AddToViewport` _output_get 0))

(event `Q_Hit`
  ;[1 1 1] Q
  (`Image.SetColorAndOpacity` (`/Game/BluePrint/UI/SkillUIWidget.Q_SkillImage_2` (`self.SkillUIReference`)) (make `LinearColor` 1.0 1.0 1.0 1.0)))

(event `ResetWSkillCoolTime`
  ;[1 1 1] W
  (set `self.CanUseSkill_W` true))

(event `Key|W`
  (params (Key :type "Key Structure"))
  (bind _returnvalue (`self.K2_GetActorLocation`))
  (bind _capsulecomponent (`self.CapsuleComponent`))
  (bind _normalattackdelay (`self.NormalAttackDelay`))
  (bind _skilluireference (`self.SkillUIReference`))
  (bind (_bblockinghit _binitialoverlap _time _distance _location _impactpoint _normal _impactnormal _physmat _hitactor) (`GameplayStatics.BreakHitResult` (`PlayerController.GetHitResultUnderCursorByChannel` (`GameplayStatics.GetPlayerController` 0) "TraceTypeQuery1" true)))
  ;[1 1 1] W
  (:`Pressed`
    (if (`self.IsUseW`)
      ;;[1 1 1] 공속 증가
      (set `self.NormalAttackDelay` (* _normalattackdelay (`self.W_SupplyAttackSpeed`)))
      (set `self.IsUseW` false)
      (`|ExecutionSequence`
        (:`then_0`
          (`KismetSystemLibrary.Delay` 3.0)
          (set `self.NormalAttackDelay` _normalattackdelay))
        (:`then_1`
          (`Image.SetColorAndOpacity` (`/Game/BluePrint/UI/SkillUIWidget.W_SkillImage_2` (`self.SkillUIReference`)) (make `LinearColor` 1.0 1.0 1.0))))
      (elif (`self.CanUseSkill_W`)
        (`GameplayStatics.SpawnDecalAtLocation` "/Engine/VREditor/LaserPointer/TranslucentHoverMaterial.TranslucentHoverMaterial" (100.0 100.0 100.0) (`SceneComponent.K2_GetComponentLocation` (`self.CapsuleComponent`)) (struct :`Pitch` -90.0) 2.0)
        (if (== _hitactor self)
          (`self.PlayAnimMontage` "/Game/BluePrint/LeeSin/Animation/LeeSin_WSkill_Me_AniMontage.LeeSin_WSkill_Me_AniMontage" 1.5)
          (set `self.IsUseW` true)
          (set `self.CanUseSkill_W` false :!label _label_2)
          (`KismetSystemLibrary.K2_SetTimer` null "ResetWSkillCoolTime" (`self.Skill_W_CoolTime`))
          (`/Game/BluePrint/UI/SkillUIWidget.StartWCoolDown` _skilluireference)
          (`/Game/BluePrint/UI/SkillUIWidget.UpdateCoolDown` _skilluireference)
          (`Image.SetColorAndOpacity` (`/Game/BluePrint/UI/SkillUIWidget.W_SkillImage_2` (`self.SkillUIReference`)) (make `LinearColor` 1.0 1.0 1.0 1.0))
          (else
            (bind _asally (cast `/Game/BluePrint/Ally/Ally` _hitactor))
            (bind _returnvalue_2 (`self.K2_GetActorLocation` _asally))
            (if (<= (`KismetMathLibrary.VSize` (- _returnvalue_2 _returnvalue)) (`self.W_MaxRange`))
              (bind (_returnvalue_roll _returnvalue_pitch _returnvalue_yaw) (`KismetMathLibrary.BreakRotator` (`KismetMathLibrary.FindLookAtRotation` _returnvalue _returnvalue_2)))
              (bind _returnvalue_3 (`KismetMathLibrary.MakeRotator` 0.0 0.0 _returnvalue_yaw))
              (`self.K2_SetActorRotation` _returnvalue_3)
              (`self.PlayAnimMontage` "/Game/BluePrint/LeeSin/Animation/LeeSin_WSkill_Ally_AniMontage.LeeSin_WSkill_Ally_AniMontage" 0.5)
              (`KismetSystemLibrary.MoveComponentTo` _capsulecomponent _returnvalue_2 _returnvalue_3 true false 0.3)
              (`|ExecutionSequence`
                (:`then_0`
                  (`MovementComponent.StopMovementImmediately` (`self.CharacterMovement`))
                  (set `self.IsUseW` true)
                  ;;[1 1 1] 자신, 아군 이펙트 생성
                  (`|ExecutionSequence`
                    (:`then_0`
                      (`GameplayStatics.SpawnEmitterAttached` "/Game/FXVarietyPack/Particles/P_ky_shootingStar1.P_ky_shootingStar1" _capsulecomponent))
                    (:`then_1`
                      (`GameplayStatics.SpawnEmitterAttached` "/Game/FXVarietyPack/Particles/P_ky_shootingStar1.P_ky_shootingStar1" (`Actor.RootComponent` _asally)))))
                (:`then_1`
                  (`self.PlayAnimMontage` "/Game/BluePrint/LeeSin/Animation/LeeSin_WSkill_Finish_AniMontage.LeeSin_WSkill_Finish_AniMontage" 1.5))
                (:`then_2`
                  (goto _label_2))))))
        (else
          (`KismetSystemLibrary.PrintText` "W스킬 쿨타임"))))))

(event `Key|E`
  (params (Key :type "Key Structure"))
  (bind _returnvalue (`self.K2_GetActorLocation`))
  (bind _skilluireference (`self.SkillUIReference`))
  ;[1 1 1] E
  (:`Pressed`
    (if (`self.IsUseE`)
      (`|ExecutionSequence`
        (:`then_0`
          (for _array_element (stale _output_get)
            (bind _movespeed (`/Game/BluePrint/Enemy/Char_Enemy.moveSpeed` _array_element))
            (set `/Game/BluePrint/Enemy/Char_Enemy.moveSpeed` (* _movespeed 0.5) _array_element)
            (set `self.IsUseE` false)
            (`KismetSystemLibrary.Delay` 3.0)
            (set `/Game/BluePrint/Enemy/Char_Enemy.moveSpeed` _movespeed _array_element)))
        (:`then_1`
          (`self.PlayAnimMontage` "/Game/BluePrint/LeeSin/Animation/LeeSin_ESkill_Slow_AniMontage.LeeSin_ESkill_Slow_AniMontage")
          (`Image.SetColorAndOpacity` (`/Game/BluePrint/UI/SkillUIWidget.E_SkillImage_2` (`self.SkillUIReference`)) (make `LinearColor` 0.0))))
      (elif (`self.CanUseSkill_E`)
        (bind _outhits (`KismetSystemLibrary.SphereTraceMultiForObjects` _returnvalue _returnvalue 150.0 (`|MakeArray` "ObjectTypeQuery8" :!type "EObjectTypeQuery Enum")))
        (`|ExecutionSequence`
          (:`then_0`
            (for _array_element_2 _outhits
              (bind _aschar_enemy (cast `/Game/BluePrint/Enemy/Char_Enemy` (`.HitActor` (`GameplayStatics.BreakHitResult` _array_element_2))))
              (`|ExecutionSequence`
                (:`then_0`
                  (`GameplayStatics.ApplyDamage` _aschar_enemy 5.0 null _aschar_enemy)
                  (set `self.IsUseE` true)
                  (`Image.SetColorAndOpacity` (`/Game/BluePrint/UI/SkillUIWidget.E_SkillImage_2` (`self.SkillUIReference`)) (make `LinearColor` 1.0 1.0 1.0 1.0)))
                (:`then_1`
                  (bind _output_get (set `self.E_HitEnemies` (`|MakeArray` _aschar_enemy))))
                (:`then_2`
                  (`GameplayStatics.SpawnEmitterAttached` "/Game/FXVarietyPack/Particles/P_ky_hit2.P_ky_hit2" (`Actor.RootComponent` _aschar_enemy)))))
            (`GameplayStatics.SpawnEmitterAttached` "/Game/FXVarietyPack/Particles/P_ky_lightning2.P_ky_lightning2" (`self.CapsuleComponent`)))
          (:`then_1`
            (`self.PlayAnimMontage` "/Game/BluePrint/LeeSin/Animation/LeeSin_ESkill_AniMontage.LeeSin_ESkill_AniMontage" 3.0)
            (set `self.CanUseSkill_E` false)
            (`KismetSystemLibrary.K2_SetTimer` null "ResetESkillCoolTime" (`self.Skill_E_CoolTime`))
            (`/Game/BluePrint/UI/SkillUIWidget.StartECoolDown` _skilluireference)
            (`/Game/BluePrint/UI/SkillUIWidget.UpdateCoolDown` _skilluireference)))
        (else
          (`KismetSystemLibrary.PrintText` "E스킬 쿨타임"))))))

(event `ResetESkillCoolTime`
  ;[1 1 1] E
  (set `self.CanUseSkill_E` true))

(event `ResetRSkillCoolTime`
  ;[1 1 1] R
  (set `self.CanUseSkill_R` true))

(event `Key|R`
  (params (Key :type "Key Structure"))
  (bind _returnvalue (`self.K2_GetActorLocation`))
  (bind _skilluireference (`self.SkillUIReference`))
  (bind (_bblockinghit _binitialoverlap _time _distance _location _impactpoint _normal _impactnormal _physmat _hitactor) (`GameplayStatics.BreakHitResult` (`PlayerController.GetHitResultUnderCursorByChannel` (`GameplayStatics.GetPlayerController` 0) "TraceTypeQuery1" true)))
  ;[1 1 1] R
  (:`Pressed`
    (if (`self.CanUseSkill_R`)
      (bind _aschar_enemy (cast `/Game/BluePrint/Enemy/Char_Enemy` _hitactor))
      (bind _output_get (set `self.TargetEnemy` _aschar_enemy))
      (if (== _hitactor _output_get)
        (bind _returnvalue_2 (`self.K2_GetActorLocation` _output_get))
        (bind _returnvalue_3 (- _returnvalue_2 _returnvalue))
        ;;[1 1 1] 거리 비교
        (if (<= (`KismetMathLibrary.VSize` _returnvalue_3) (`self.R_MaxRange`))
          (`|ExecutionSequence`
            (:`then_0`
              (bind (_returnvalue_roll _returnvalue_pitch _returnvalue_yaw) (`KismetMathLibrary.BreakRotator` (`KismetMathLibrary.FindLookAtRotation` _returnvalue _returnvalue_2)))
              (`self.K2_SetActorRotation` (`KismetMathLibrary.MakeRotator` 0.0 0.0 _returnvalue_yaw))
              (`self.PlayAnimMontage` "/Game/BluePrint/LeeSin/Animation/LeeSin_RSkill_AniMontage.LeeSin_RSkill_AniMontage" 0.6)
              (`GameplayStatics.ApplyDamage` _output_get 10.0)
              (set `/Game/BluePrint/Enemy/Char_Enemy.is_R_Airborne` true _output_get)
              (`|ExecutionSequence`
                (:`then_0`
                  (bind _capsulecomponent (`Character.CapsuleComponent` _output_get))
                  (bind (_returnvalue_x _returnvalue_y) (`KismetMathLibrary.BreakVector` (+ (* (`KismetMathLibrary.Normal` _returnvalue_3) (`self.R_Force`)) _returnvalue_2)))
                  (bind (_returnvalue_x_2 _returnvalue_y_2 _returnvalue_z) (`KismetMathLibrary.BreakVector` (`self.K2_GetActorLocation` _output_get)))
                  (`KismetSystemLibrary.MoveComponentTo` _capsulecomponent (`KismetMathLibrary.MakeVector` _returnvalue_x _returnvalue_y _returnvalue_z) (struct) false false 1.2))
                (:`then_1`
                  (bind _outhits (`KismetSystemLibrary.SphereTraceMultiForObjects` _returnvalue_2 (`KismetMathLibrary.MakeVector` _returnvalue_x _returnvalue_y _returnvalue_z) 100.0 (`|MakeArray` "ObjectTypeQuery8" :!type "EObjectTypeQuery Enum")))
                  (for _array_element _outhits
                    (bind _aschar_enemy_2 (cast `/Game/BluePrint/Enemy/Char_Enemy` (`.HitActor` (`GameplayStatics.BreakHitResult` _array_element))))
                    (`|ExecutionSequence`
                      (:`then_0`
                        (`PrimitiveComponent.AddImpulse` (`Character.CapsuleComponent` _aschar_enemy_2) (0.0 0.0 0.0) "None" false)
                        (`GameplayStatics.ApplyDamage` _aschar_enemy_2 50.0))
                      (:`then_1`
                        (bind _output_get_2 (set `/Game/BluePrint/Enemy/Char_Enemy.enemy_position` (`self.K2_GetActorLocation` _aschar_enemy_2) _aschar_enemy_2))))))
                (:`then_2`
                  (`GameplayStatics.SpawnEmitterAttached` "/Game/FXVarietyPack/Particles/P_ky_ThunderBallHit.P_ky_ThunderBallHit" _capsulecomponent))))
            (:`then_1`
              (`PrimitiveComponent.SetPhysicsLinearVelocity` _capsulecomponent (0.0 0.0 0.0) false "None" :!label _label_3)
              (`PrimitiveComponent.AddImpulse` _capsulecomponent (0.0 0.0 0.0) "None" false)
              (`KismetSystemLibrary.Delay` 1.0)
              (`PrimitiveComponent.SetPhysicsLinearVelocity` _capsulecomponent (0.0 0.0 0.0) false "None")
              (set `/Game/BluePrint/Enemy/Char_Enemy.is_R_Airborne` false _output_get))
            (:`then_2`
              (set `self.CanUseSkill_R` false)
              (`KismetSystemLibrary.K2_SetTimer` null "ResetRSkillCoolTime" (`self.Skill_R_CoolTime`))
              (`/Game/BluePrint/UI/SkillUIWidget.StartRCoolDown` _skilluireference)
              (`/Game/BluePrint/UI/SkillUIWidget.UpdateCoolDown` _skilluireference)))))
      (else
        (`KismetSystemLibrary.PrintText` "R스킬 쿨타임")))))

(event `Reset Airborne`
  ;[1 1 1] R
  (`self.K2_SetActorLocation` (stale `Key|R` _aschar_enemy_2) (stale `Key|R` _output_get_2) false false))

(event `Airborne`
  ;[1 1 1] R
  (goto _label_3))

(fn `UserConstructionScript`)