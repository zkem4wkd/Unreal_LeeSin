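; BP_Cube is an actor that moves its Sphere component up and down once along Z when play begins.
; BeginPlay calls the custom event 올라감 (going up), which plays a timeline whose track drives the sphere's relative transform.
; When it finishes, a short delay leads into a second timeline, played in reverse from the end, driving the same Z value.
; TestFunction and a few disconnected nodes are unused scraps.
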(event `self.ReceiveBeginPlay`
  (`self.올라감`))

(event `올라감`
  (bind _sphere (`self.Sphere`))
  (bind (_direction `_업다운_타임라인`) (`Timeline|타임라인`)
    (:`Update`
      (`SceneComponent.K2_SetRelativeTransform` _sphere (`KismetMathLibrary.MakeTransform` (`KismetMathLibrary.MakeVector` 0.0 0.0 `_업다운_타임라인`)) false false))
    (:`Finished`
      ;[1 1 1] 광역 선택하고 C
      (`KismetSystemLibrary.Delay` 1.0)
      (bind (_direction_2 `_업다운_타임라인_2`) (`Timeline|타임라인_0` :!via `ReverseFromEnd`)
        (:`Update`
          (`SceneComponent.K2_SetRelativeTransform` _sphere (`KismetMathLibrary.MakeTransform` (`KismetMathLibrary.MakeVector` 0.0 0.0 `_업다운_타임라인_2`)) false false))))))

(fn `Test_Function`
  (`SceneComponent.K2_SetRelativeTransform` (`self.Sphere`) (`KismetMathLibrary.MakeTransform` (0.0 0.0 0.0)) false false))

(fn `UserConstructionScript`)